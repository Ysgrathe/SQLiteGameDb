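; BP_2DThingArray is a fixed-size 2D container of Thing elements backed by one flat array.
; Init stores both dimensions, then clears and resizes the array to their product.
; Get and set share an index helper computing D1 * SizeD1 + D2, a stride that suits only square grids.
; The helper checks only the flat index against the array's upper bound, logging when it is out of range.
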(fn `ArrayIndexFromDimensions`
  (params (D1 :type Integer) (D2 :type Integer))
  (returns (ArrayIndex :type Integer))
  (bind _returnvalue (+ (* D1 (`self.SizeD1`)) D2))
  (if (< _returnvalue (`KismetArrayLibrary.Array_Length` (`self.InternalArray`)))
    (return _returnvalue)
    (else
      (`KismetSystemLibrary.LogString` "Requested Index Out Of Bounds!"))))

(fn `GetElement2D`
  (params (D1 :type Integer) (D2 :type Integer))
  (returns (Thing :type "/Game/Blueprints/BP_Thing Object Reference"))
  (return (`|GetArrayItem` (`self.InternalArray`) (`self.ArrayIndexFromDimensions` D1 D2))))

(fn `Init`
  (params (InSizeD1 :type Integer) (InSizeD2 :type Integer))
  (set `self.SizeD1` InSizeD1)
  (set `self.SizeD2` InSizeD2)
  (bind _output_get (set `self.ArraySize` (* (`self.SizeD1`) (`self.SizeD2`))))
  (`KismetArrayLibrary.Array_Clear` (`self.InternalArray`))
  (`KismetArrayLibrary.Array_Resize` (`self.InternalArray`) _output_get))

(fn `SetElement2D`
  (params (D1 :type Integer) (D2 :type Integer) (Thing :type "/Game/Blueprints/BP_Thing Object Reference"))
  (`KismetArrayLibrary.Array_Set` (`self.InternalArray`) (`self.ArrayIndexFromDimensions` D1 D2) Thing))