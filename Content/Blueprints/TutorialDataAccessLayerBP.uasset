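; Tutorial data access layer that reads backgrounds, character classes and weapon types from a database and saves the player's chosen background, class and name.
; Startup loads statements through the inherited QueryManager, and each function looks up a prepared statement by name, binds parameters and executes it.
; Select results pass through a shared converter that maps generic rows into simple ID, name, description and color structs, defaulting the color when its fields are missing.
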(event `self.Startup`
  (params (DatabaseFilePath :type String) (Config :type "GameDbConfig Structure (by ref)"))
  (`PreparedStatementManager.LoadStatements` (`self.QueryManager`)))

(fn `GetBackgroundList`
  (returns (Data :type "Array of /Game/Blueprints/SimpleDataItemBP Structure"))
  (locals (PreparedStatement :type "DbStatement Object Reference") (ResultData :type "QueryResult Structure"))
  (bind (_statement _isvalid) (`self.GetQuery` "GetBackgroundList"))
  (if _isvalid
    (set `local.PreparedStatement` _statement)
    (bind _returnvalue (`DbStatement.ExecuteSelect` (`local.PreparedStatement`)))
    (bind _output_get (set `local.ResultData` _returnvalue))
    (bind _simplearray (`self.QueryResultToSimpleArray` _output_get))
    (return _simplearray)))

(fn `GetClassesForBackground`
  (params (BackgroundID :type Integer))
  (returns (Data :type "Array of /Game/Blueprints/SimpleDataItemBP Structure"))
  (locals (PreparedStatement :type "DbStatement Object Reference") (ResultData :type "QueryResult Structure"))
  (bind (_statement _isvalid) (`self.GetQuery` "GetClassesListForBackgroundID"))
  (if _isvalid
    (set `local.PreparedStatement` _statement)
    ;[1 0.3209 0.5547] Set Query Parameter Values
    (`DbStatement.SetIntParameterValue` (`local.PreparedStatement`) "@BackgroundID" BackgroundID)
    (bind _returnvalue (`DbStatement.ExecuteSelect` (`local.PreparedStatement`)))
    (bind _output_get (set `local.ResultData` _returnvalue))
    (bind _simplearray (`self.QueryResultToSimpleArray` _output_get))
    (return _simplearray)))

(fn `GetQuery`
  (params (StatementName :type String))
  (returns (Statement :type "DbStatement Object Reference") (IsValid :type Boolean))
  (bind _returnvalue (`PreparedStatementManager.FindStatement` (`self.QueryManager`) StatementName))
  (return _returnvalue (`KismetSystemLibrary.IsValid` _returnvalue)))

(fn `GetWeaponTypesForCharacterClass`
  (params (CharacterClassID :type Integer))
  (returns (Data :type "Array of /Game/Blueprints/SimpleDataItemBP Structure"))
  (locals (PreparedStatement :type "DbStatement Object Reference") (ResultData :type "QueryResult Structure"))
  (bind (_statement _isvalid) (`self.GetQuery` "GetWeaponTypesForClassID"))
  (if _isvalid
    (set `local.PreparedStatement` _statement)
    (`DbStatement.SetIntParameterValue` (`local.PreparedStatement`) "@CharacterClassID" CharacterClassID)
    (bind _returnvalue (`DbStatement.ExecuteSelect` (`local.PreparedStatement`)))
    (bind _output_get (set `local.ResultData` _returnvalue))
    (bind _simplearray (`self.QueryResultToSimpleArray` _output_get))
    (return _simplearray)))

(fn `QueryResultToSimpleArray`
  (params (QueryResult :type "QueryResult Structure"))
  (returns (SimpleArray :type "Array of /Game/Blueprints/SimpleDataItemBP Structure"))
  (locals (ResultList :type "Array of /Game/Blueprints/SimpleDataItemBP Structure") (ResultItem :type "/Game/Blueprints/SimpleDataItemBP Structure") (TmpColor :type "LinearColor Structure"))
  ;[0.3739 1 0.5374] Loop over the 'generic' query data, and create an array of a specific struct from the rows.
  (for _array_element (`.Rows` (break `QueryResult` QueryResult))
    ;[1 0.5059 0] Color from database fields - Searches for fields with base name, plus R, G, B, A
    ; And creates a linear color structure from them.
    ; A Boolean lets you know if it was successful.
    (bind (_color _returnvalue) (`GameDatabaseStatics.TryFillColor` _array_element))
    (if _returnvalue
      (set `local.TmpColor` _color)
      (else
        (set `local.TmpColor` (make `LinearColor` 0.0 0.0 0.0 1.0))))
    (bind _fields (break `QueryResultRow` _array_element))
    (bind _output_get (set `local.ResultItem` (make `/Game/Blueprints/SimpleDataItemBP` (`KismetMathLibrary.Conv_Int64ToInt` (`.IntVal` (break `QueryResultField` (`|GetArrayItem` _fields)))) (`.StrVal` (break `QueryResultField` (`|GetArrayItem` _fields 1))) (`.StrVal` (break `QueryResultField` (`|GetArrayItem` _fields 2))) (`local.TmpColor`))))
    (`KismetArrayLibrary.Array_Add` (`local.ResultList`) _output_get))
  (return (`local.ResultList`)))

(fn `SavePlayerInfo`
  (params (BackgroundID :type Integer) (CharacterClassID :type Integer) (Name :type String))
  (locals (PreparedStatement :type "DbStatement Object Reference"))
  (bind _preparedstatement (`local.PreparedStatement`))
  (bind (_statement _isvalid) (`self.GetQuery` "SavePlayerInfo"))
  (if _isvalid
    (set `local.PreparedStatement` _statement)
    (`DbStatement.SetIntParameterValue` _preparedstatement "@BackgroundID" BackgroundID)
    (`DbStatement.SetIntParameterValue` _preparedstatement "@CharacterClassID" CharacterClassID)
    (`DbStatement.SetStringParameterValue` _preparedstatement "@Name" Name)
    (`DbStatement.ExecuteAction` _preparedstatement)))